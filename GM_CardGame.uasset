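; GM_CardGame is the game mode that starts a card game.
; On BeginPlay it creates the WBP_HUD widget, stores it as MainWidget and adds it to the viewport.
; It then finds the first BP_TableEnv in the level, calls InitializeGame on it, and triggers UseCard after a one-second delay.
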(event EventBeginPlay
  (bind _returnvalue (UserInterface|CreateWidget "/Game/WidgetBlueprint/MyGameWBP/WBP_HUD.WBP_HUD_C"))
  (Variables|Default|SetMainWidget _returnvalue)
  (UserInterface|Viewport|AddtoViewport _returnvalue 0)
  (bind _outactors (Actor|GetAllActorsOfClass "/Game/Blueprint/MyGameBP/BP_TableEnv.BP_TableEnv_C"))
  (Variables|Default|SetTableEnv (Utilities|Array|Get(acopy) _outactors))
  (Default|InitializeGame (Variables|Default|GetTableEnv))
  (Utilities|FlowControl|Delay 1.0)
  (Default|UseCard (Variables|Default|GetTableEnv)))

(fn ConstructionScript)